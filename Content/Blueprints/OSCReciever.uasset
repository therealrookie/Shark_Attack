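; OSC receiver Blueprint that turns incoming network messages into shark controls, sent to actors through interface calls.
; BeginPlay starts two OSC servers on a hardcoded IP, each with its own message handler.
; The first routes by address path, triggering bites or sending X movement remapped to a signed axis with a centre dead zone.
; The second only reads a float, as its cube-positioning logic is disconnected.
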(event `self.ReceiveBeginPlay`
  (bind _returnvalue (`OSCManager.CreateOSCServer` "192.168.178.32" 8080 false true "" null))
  (bind _output_get (set `self.OSCReciever` _returnvalue))
  (clear `OSCServer.OnOscBundleReceived` _output_get)
  (add `OSCServer.OnOscMessageReceived` _output_get (`|CreateDelegate` :!event `OSCMessage`))
  (bind _returnvalue_2 (`OSCManager.CreateOSCServer` "192.168.178.32" 8020 false true "" null))
  (bind _output_get_2 (set `self.OSCReciever2` _returnvalue_2))
  (clear `OSCServer.OnOscBundleReceived` _output_get_2)
  (add `OSCServer.OnOscMessageReceived` _output_get_2 (`|CreateDelegate` :!event `OSCMessage2`)))

(event `OSCMessage`
  (params (Message :type "OSCMessage Structure (by ref)") (IPAddress :type String) (Port :type Integer))
  (bind _returnvalue (`OSCManager.GetOSCMessageAddress` Message))
  (bind _returnvalue_2 (`OSCManager.GetOSCAddressFullPath` _returnvalue))
  (switch `string` _returnvalue_2
    (:`/sharkBite`
      (bind _outactors (`GameplayStatics.GetAllActorsWithInterface` "/Game/Blueprints/OSCControlInterface.OSCControlInterface_C"))
      (message `/Game/Blueprints/OSCControlInterface.triggerSharkBite` _outactors))
    (:`/sharkMove`
      (`self.moveShark`)
      (bind _outactors_2 (`GameplayStatics.GetAllActorsWithInterface` null))
      (bind _returnvalue_3 (`KismetMathLibrary.MapRangeClamped` (stale `moveShark` _value_2) 0.0 1.0 1.0 -1.0))
      (message `/Game/Blueprints/OSCControlInterface.moveSharkX` _outactors_2 (`KismetMathLibrary.SelectFloat` 0.0 _returnvalue_3 (and (> _returnvalue_3 -0.1) (< _returnvalue_3 0.1)))))))

(event `moveShark`
  (bind _value (`OSCManager.GetFloat` (stale `OSCMessage` Message)))
  (bind _value_2 (`OSCManager.GetFloat` (stale `OSCMessage` Message) 1)))

(event `OSCMessage2`
  (params (Message :type "OSCMessage Structure (by ref)") (IPAddress :type String) (Port :type Integer))
  (bind _value (`OSCManager.GetFloat` Message)))

(fn `UserConstructionScript`)